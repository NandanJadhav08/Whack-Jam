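; BP_DuctTape is a collectible duct tape pickup that bobs between two positions until the player collects it.
; Two timelines, MoveUp and MoveDown, trigger each other endlessly from BeginPlay, lerping the DuctTape component's relative location between StartLocation and EndLocation.
; When BP_TopDownCharacter overlaps the Box, the pickup increments that character's DuctTapeCount and destroys itself.
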(event `self.ReceiveBeginPlay`
  (bind (_direction _alpha) (`Timeline|MoveUp` :!via `PlayFromStart` :!label _label)
    (:`Update`
      (`SceneComponent.K2_SetRelativeLocation` (`self.DuctTape`) (`KismetMathLibrary.VLerp` (`self.Start Location`) (`self.EndLocation`) _alpha) false false))
    (:`Finished`
      (bind (_direction_2 _alpha_2) (`Timeline|MoveDown` :!via `ReverseFromEnd`)
        (:`Update`
          (`SceneComponent.K2_SetRelativeLocation` (`self.DuctTape`) (`KismetMathLibrary.VLerp` (`self.Start Location`) (`self.EndLocation`) _alpha_2) false false))
        (:`Finished`
          (goto _label :!via `PlayFromStart`))))))

(event `self.Box.OnComponentBeginOverlap`
  (params (OverlappedComponent :type "PrimitiveComponent Object Reference") (OtherActor :type "Actor Object Reference") (OtherComp :type "PrimitiveComponent Object Reference") (OtherBodyIndex :type Integer) (bFromSweep :type Boolean) (SweepResult :type "HitResult Structure (by ref)"))
  (bind _asbp_top_down_character (cast `/Game/Blueprints/BP_TopDownCharacter` OtherActor))
  (bind _result (`/Engine/EditorBlueprintResources/StandardMacros.IncrementInt` (`/Game/Blueprints/BP_TopDownCharacter.DuctTapeCount` _asbp_top_down_character))
    (:`  `
      (set `/Game/Blueprints/BP_TopDownCharacter.DuctTapeCount` _result _asbp_top_down_character)
      (`self.K2_DestroyActor`))))

(fn `UserConstructionScript`)