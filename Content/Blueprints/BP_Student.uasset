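; BP_Student is a student that ends the player's run on overlap with its Caught volume, calling the character's lose event, stopping movement and playing a snitch sound.
; An interaction volume registers it as the character's interactable and shows a text prompt when the player carries duct tape.
; Its Taped event, valid in range and only once, destroys the catch volume and cone, reveals the tape and plays a random duct-tape sound.
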(event `self.Caught.OnComponentBeginOverlap`
  (params (OverlappedComponent :type "PrimitiveComponent Object Reference") (OtherActor :type "Actor Object Reference") (OtherComp :type "PrimitiveComponent Object Reference") (OtherBodyIndex :type Integer) (bFromSweep :type Boolean) (SweepResult :type "HitResult Structure (by ref)"))
  (bind _asbp_top_down_character (cast `/Game/Blueprints/BP_TopDownCharacter` OtherActor))
  (`/Game/Blueprints/BP_TopDownCharacter.LoseEvent` _asbp_top_down_character)
  (`/Game/Blueprints/BP_TopDownCharacter.StopAllMovement` _asbp_top_down_character)
  (`GameplayStatics.PlaySound2D` "/Game/SFX/Snitch.Snitch" 1.0 1.0 0.0 null null))

(event `self.InteractCollision.OnComponentBeginOverlap`
  (params (OverlappedComponent :type "PrimitiveComponent Object Reference") (OtherActor :type "Actor Object Reference") (OtherComp :type "PrimitiveComponent Object Reference") (OtherBodyIndex :type Integer) (bFromSweep :type Boolean) (SweepResult :type "HitResult Structure (by ref)"))
  (bind _asbp_top_down_character (cast `/Game/Blueprints/BP_TopDownCharacter` OtherActor))
  (bind _output_get (set `self.Character` _asbp_top_down_character))
  (set `self.CanInteract` true)
  (set `/Game/Blueprints/BP_TopDownCharacter.InteractableObject` self _asbp_top_down_character)
  (if (> (`/Game/Blueprints/BP_TopDownCharacter.DuctTapeCount` _output_get) 0)
    (if (not (`self.IsTaped`))
      (`SceneComponent.SetVisibility` (`self.TextRender`) true false))))

(event `self.InteractCollision.OnComponentEndOverlap`
  (params (OverlappedComponent :type "PrimitiveComponent Object Reference") (OtherActor :type "Actor Object Reference") (OtherComp :type "PrimitiveComponent Object Reference") (OtherBodyIndex :type Integer))
  (cast `/Game/Blueprints/BP_TopDownCharacter` OtherActor)
  (set `self.CanInteract` false)
  (`SceneComponent.SetVisibility` (`self.TextRender`) false false))

(event `Taped`
  (if (`self.CanInteract`)
    (if (not (`self.IsTaped`))
      (`ActorComponent.K2_DestroyComponent` (`self.Caught`))
      (`ActorComponent.K2_DestroyComponent` (`self.Cone`))
      (set `self.IsTaped` true)
      (`SceneComponent.SetVisibility` (`self.TextRender`) false false)
      (`SceneComponent.SetVisibility` (`self.Tape`) true false)
      (switch `int` (`KismetMathLibrary.RandomIntegerInRange` 0 2)
        (:`0`
          (`GameplayStatics.PlaySoundAtLocation` "/Game/SFX/DuctTapeSFX1.DuctTapeSFX1" (`self.K2_GetActorLocation`) (struct) 1.0 1.0 0.0 null null null null))
        (:`1`
          (`GameplayStatics.PlaySoundAtLocation` "/Game/SFX/DuctTapeSFX2.DuctTapeSFX2" (`self.K2_GetActorLocation`) (struct) 1.0 1.0 0.0 null null null null))
        (:`2`
          (`GameplayStatics.PlaySoundAtLocation` "/Game/SFX/DuctTapeSFX3.DuctTapeSFX3" (`self.K2_GetActorLocation`) (struct) 1.0 1.0 0.0 null null null null))))))

(fn `UserConstructionScript`)