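; BP_Teacher is a teacher actor that makes the player lose on contact and can be neutralized by taping.
; Overlapping its Caught component with BP_TopDownCharacter calls that character's LoseEvent and stops its movement.
; The Taped event, gated by CanInteract and a one-shot IsTaped flag, destroys Caught, hides the text render and prints a debug message.
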(event `self.Caught.OnComponentBeginOverlap`
  (params (OverlappedComponent :type "PrimitiveComponent Object Reference") (OtherActor :type "Actor Object Reference") (OtherComp :type "PrimitiveComponent Object Reference") (OtherBodyIndex :type Integer) (bFromSweep :type Boolean) (SweepResult :type "HitResult Structure (by ref)"))
  (bind _asbp_top_down_character (cast `/Game/Blueprints/BP_TopDownCharacter` OtherActor))
  (`/Game/Blueprints/BP_TopDownCharacter.LoseEvent` _asbp_top_down_character)
  (`/Game/Blueprints/BP_TopDownCharacter.StopAllMovement` _asbp_top_down_character))

(event `Taped`
  (if (`self.CanInteract`)
    (if (not (`self.IsTaped`))
      (`ActorComponent.K2_DestroyComponent` (`self.Caught`))
      (set `self.IsTaped` true)
      (`SceneComponent.SetVisibility` (`self.TextRender`) false false)
      (`KismetSystemLibrary.PrintString` "TAPED" true true (struct :`G` 1.0 :`B` 0.051414 :`A` 1.0)))))

(fn `UserConstructionScript`)